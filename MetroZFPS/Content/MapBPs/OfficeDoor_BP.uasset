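; Locked office door that the player opens with the Interact input by spending one key from the first-person character.
; Overlapping the trigger enables input and opens a gate, with no end-overlap handler to close it again.
; A successful unlock decrements Keys, swings the door by timeline-driven rotator lerp and destroys the trigger.
; Also supplies an "Open" interaction prompt attached to that trigger.
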(event `self.ReceiveBeginPlay`
  (set `self.DoorOrigin` (`SceneComponent.RelativeRotation` (`self.Door`))))

(event `Open Doors`
  (bind (_direction _0_to1) (`Timeline|Timeline_0`)
    (:`Update`
      (`SceneComponent.K2_SetRelativeRotation` (`self.Door`) (`KismetMathLibrary.RLerp` (`self.DoorOrigin`) (struct :`Yaw` -90.0) _0_to1 true) false false))))

(event `InputAction|Interact`
  (params (Key :type "Key Structure"))
  (bind _as_first_person_character (`self.As First Person Character`))
  (:`Pressed`
    (`/Engine/EditorBlueprintResources/StandardMacros.Gate` true :!label _label
      (:`Exit`
        (bind _asfirst_person_character (cast `/Game/FirstPersonBP/Blueprints/FirstPersonCharacter` (`GameplayStatics.GetPlayerCharacter` 0)))
        (bind _output_get (set `self.As First Person Character` _asfirst_person_character))
        (if (> (`/Game/FirstPersonBP/Blueprints/FirstPersonCharacter.Keys` _output_get) 0)
          (set `/Game/FirstPersonBP/Blueprints/FirstPersonCharacter.Keys` (- (`/Game/FirstPersonBP/Blueprints/FirstPersonCharacter.Keys` _as_first_person_character) 1) _as_first_person_character)
          (`self.Open Doors`)
          (`ActorComponent.K2_DestroyComponent` (`self.Overlap`)))))))

(event `self.Overlap.OnComponentBeginOverlap`
  (params (OverlappedComponent :type "PrimitiveComponent Object Reference") (OtherActor :type "Actor Object Reference") (OtherComp :type "PrimitiveComponent Object Reference") (OtherBodyIndex :type Integer) (bFromSweep :type Boolean) (SweepResult :type "HitResult Structure (by ref)"))
  (if (== OtherActor (`GameplayStatics.GetPlayerCharacter` 0))
    (`self.EnableInput` (`GameplayStatics.GetPlayerController` 0))
    (cast `/Game/FirstPersonBP/Blueprints/FirstPersonCharacter` OtherActor)
    (goto _label :!via `Open`)))

(fn `GetInteractionText`
  (returns (Text :type Text))
  (return "Open"))

(fn `GetInteractionTextAttach`
  (returns (AttachComponent :type "SceneComponent Object Reference"))
  (return (`self.Overlap`)))

(fn `UserConstructionScript`
  (`parent.UserConstructionScript`))