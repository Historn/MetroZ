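; ElectricityKey_BP is a pickup actor for an electricity key that the player collects with the Interact input.
; When the player character overlaps PickOverlap, the actor enables input and opens a gate on the Interact action.
; An Interact press through the open gate increments KeyElectricity on FirstPersonCharacter and destroys the key.
; No end-overlap handler closes the gate or disables input, so the key stays collectable after the player walks away.
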(event `InputAction|Interact`
  (params (Key :type "Key Structure"))
  (:`Pressed`
    (`/Engine/EditorBlueprintResources/StandardMacros.Gate` true :!label _label
      (:`Exit`
        (bind _asfirst_person_character (cast `/Game/FirstPersonBP/Blueprints/FirstPersonCharacter` (`GameplayStatics.GetPlayerCharacter` 0)))
        (`/Engine/EditorBlueprintResources/StandardMacros.IncrementInt` (`/Game/FirstPersonBP/Blueprints/FirstPersonCharacter.KeyElectricity` _asfirst_person_character)
          (:`  `
            (`self.K2_DestroyActor`)))))))

(event `self.PickOverlap.OnComponentBeginOverlap`
  (params (OverlappedComponent :type "PrimitiveComponent Object Reference") (OtherActor :type "Actor Object Reference") (OtherComp :type "PrimitiveComponent Object Reference") (OtherBodyIndex :type Integer) (bFromSweep :type Boolean) (SweepResult :type "HitResult Structure (by ref)"))
  (if (== OtherActor (`GameplayStatics.GetPlayerCharacter` 0))
    (`self.EnableInput` (`GameplayStatics.GetPlayerController` 0))
    (cast `/Game/FirstPersonBP/Blueprints/FirstPersonCharacter` OtherActor)
    (goto _label :!via `Open`)))

(fn `UserConstructionScript`
  (`parent.UserConstructionScript`))