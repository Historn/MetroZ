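; BP_Zombie is an AI-controlled zombie character that varies per instance and can be killed.
; On BeginPlay it randomizes mesh scale on each axis, facing yaw and walk speed.
; Its Kill event stops the AI brain, disables capsule and mesh collision and plays the death animation.
; After a delay it broadcasts the OnKilled dispatcher and destroys itself.
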(event `self.ReceiveBeginPlay`
  (bind _returnvalue (`KismetMathLibrary.RandomFloatInRange` 7.9 8.1))
  (`SceneComponent.SetWorldScale3D` (`self.Mesh`) (`KismetMathLibrary.MakeVector` _returnvalue _returnvalue _returnvalue))
  (`self.K2_SetActorRotation` (`KismetMathLibrary.MakeRotator` 0.0 0.0 (`KismetMathLibrary.RandomFloatInRange` 0.0 360.0)))
  (set `CharacterMovementComponent.MaxWalkSpeed` (`KismetMathLibrary.RandomFloatInRange` 300.0 500.0) (`self.CharacterMovement`)))

(event `Kill`
  (`BrainComponent.StopLogic` (`AIController.BrainComponent` (`AIBlueprintHelperLibrary.GetAIController` self)) "")
  (`PrimitiveComponent.SetCollisionProfileName` (`self.CapsuleComponent`) "NoCollision" true)
  (`PrimitiveComponent.SetCollisionProfileName` (`self.Mesh`) "NoCollision" true)
  (`SkeletalMeshComponent.PlayAnimation` (`self.Mesh`) "/Game/Zombis/Zombies/Animaciones/zombie_death.zombie_death" false)
  (`KismetSystemLibrary.Delay` 6.0)
  (`self.OnKilled` self)
  (`self.K2_DestroyActor`))

(fn `UserConstructionScript`)