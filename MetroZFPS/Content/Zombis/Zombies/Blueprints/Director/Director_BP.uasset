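; Director that tracks the zombie population and caps how many horde spawners can add.
; On BeginPlay it registers existing zombies and horde spawners, binding to their kill and spawn-request events.
; Spawn requests create zombies at random reachable points near the requested location, up to MaxZombies, and register each success.
; Tick prints the live zombie count as debug output.
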(event `self.ReceiveBeginPlay`
  (`|ExecutionSequence`
    (:`then_0`
      (bind _outactors (`GameplayStatics.GetAllActorsOfClass` "/Game/Zombis/Zombies/Blueprints/BP_Zombie.BP_Zombie_C"))
      (for _array_element _outactors
        (`self.OnZombieSpawned` _array_element)))
    (:`then_1`
      (bind _outactors_2 (`GameplayStatics.GetAllActorsOfClass` "/Game/Zombis/Zombies/Blueprints/Director/HorderSpawner_BP.HorderSpawner_BP_C"))
      (for _array_element_2 _outactors_2
        (`self.OnHordeSpawnerSpawed` _array_element_2)))))

(event `self.ReceiveTick`
  (params (DeltaSeconds :type "Float (single-precision)"))
  (`KismetSystemLibrary.PrintString` (`KismetStringLibrary.Concat_StrStr` "Num Zombies" (`KismetStringLibrary.Conv_IntToString` (`KismetArrayLibrary.Array_Length` (`self.Zombie`)))) true true (struct :`G` 0.66 :`B` 1.0 :`A` 1.0) 0.0))

(fn `OnHordeSpawnerSpawed`
  (params (HordeSpawner :type "/Game/Zombis/Zombies/Blueprints/Director/HorderSpawner_BP Object Reference"))
  (`KismetArrayLibrary.Array_Add` (`self.Horde Spawners`) HordeSpawner)
  (add `/Game/Zombis/Zombies/Blueprints/Director/HorderSpawner_BP.RequestSpawn` HordeSpawner (`|CreateDelegate` :!event `OnZombieSpawnRequested`)))

(fn `OnZombieKilled`
  (params (Zombie :type "/Game/Zombis/Zombies/Blueprints/BP_Zombie Object Reference"))
  (`KismetArrayLibrary.Array_RemoveItem` (`self.Zombie`) Zombie))

(fn `OnZombieSpawned`
  (params (Zombie :type "/Game/Zombis/Zombies/Blueprints/BP_Zombie Object Reference"))
  (`KismetArrayLibrary.Array_Add` (`self.Zombie`) Zombie)
  (add `/Game/Zombis/Zombies/Blueprints/BP_Zombie.OnKilled` Zombie (`|CreateDelegate` :!event `OnZombieKilled`)))

(fn `OnZombieSpawnRequested`
  (params (Count :type Integer) (Location :type "Vector Structure"))
  (for _ (range 1 (+ (`KismetMathLibrary.Min` Count (- (`self.MaxZombies`) (`KismetArrayLibrary.Array_Length` (`self.Zombie`)))) 1))
    (bind _returnvalue (`|SpawnActorFromClass` "/Game/Zombis/Zombies/Blueprints/BP_Zombie.BP_Zombie_C" (`KismetMathLibrary.MakeTransform` (+ (`NavigationSystemV1.K2_GetRandomReachablePointInRadius` (`local.Location`) 200.0 null null) (0.0 0.0 75.0))) "AdjustIfPossibleButDontSpawnIfColliding" "OverrideRootScale" null null))
    (`/Engine/EditorBlueprintResources/StandardMacros.IsValid` _returnvalue
      (:`Is Valid`
        (`self.OnZombieSpawned` _returnvalue)))))

(fn `UserConstructionScript`)